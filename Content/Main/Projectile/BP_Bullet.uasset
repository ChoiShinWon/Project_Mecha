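; BP_Bullet is a projectile actor that applies Gameplay Ability System damage on impact.
; BeginPlay makes the collision Sphere the component driven by ProjectileMovement, and the Sphere's hit event handles impacts.
; A target with an ability system component receives GE_BulletDamage from the instigator's component plus a small NA_Explosion, while other hits spawn NA_Explosion3.
; The bullet destroys itself after any hit, skipping damage and effects on its owner.
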(event `self.ReceiveBeginPlay`
  (`MovementComponent.SetUpdatedComponent` (`self.ProjectileMovement`) (`self.Sphere`)))

(event `self.ReceiveHit`
  (params (MyComp :type "PrimitiveComponent Object Reference") (Other :type "Actor Object Reference") (OtherComp :type "PrimitiveComponent Object Reference") (bSelfMoved :type Boolean) (HitLocation :type "Vector Structure") (HitNormal :type "Vector Structure") (NormalImpulse :type "Vector Structure") (Hit :type "HitResult Structure (by ref)")))

(event `self.Sphere.OnComponentHit`
  (params (HitComponent :type "PrimitiveComponent Object Reference") (OtherActor :type "Actor Object Reference") (OtherComp :type "PrimitiveComponent Object Reference") (NormalImpulse :type "Vector Structure") (Hit :type "HitResult Structure (by ref)"))
  (bind (_bblockinghit _binitialoverlap _time _distance _location _impactpoint _normal _impactnormal _physmat _hitactor) (`GameplayStatics.BreakHitResult` Hit))
  (if (== (`self.GetOwner`) _hitactor)
    (`self.K2_DestroyActor`)
    (else
      (bind _output_get (set `self.TargetASC` (`AbilitySystemBlueprintLibrary.GetAbilitySystemComponent` _hitactor)))
      ;[1 1 1] 맞은게 적인지
      (`/Engine/EditorBlueprintResources/StandardMacros.IsValid` _output_get
        (:`Is Valid`
          (`AbilitySystemComponent.BP_ApplyGameplayEffectToTarget` :`self` (`AbilitySystemBlueprintLibrary.GetAbilitySystemComponent` (`self.GetInstigator`)) :`GameplayEffectClass` "/Game/Main/GE/Damage/Player/GE_BulletDamage.GE_BulletDamage_C" :`Target` (`self.TargetASC`) :`Level` 1.0)
          (`|SpawnActorFromClass` "/Game/Main/Niagara/NA_Explosion.NA_Explosion_C" (`KismetMathLibrary.MakeTransform` _impactpoint (struct) (0.2 0.2 0.2)) "Undefined" "MultiplyWithRoot" null null)
          (`self.K2_DestroyActor`))
        (:`Is Not Valid`
          (`|SpawnActorFromClass` "/Game/Main/Niagara/NA_Explosion3.NA_Explosion3_C" (`KismetMathLibrary.MakeTransform` _impactpoint (struct) (0.2 0.2 0.2)) "Undefined" "MultiplyWithRoot" null null)
          (`self.K2_DestroyActor`))))))

(fn `UserConstructionScript`)