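; Boss missile rain projectile that damages the player mecha on impact through the Gameplay Ability System.
; Its sphere ignores the owner when moving, and any hit destroys the projectile.
; On hitting a BP_MechaCharacter other than the owner, it spawns an impact particle actor.
; If that target has an ability system component, it also plays a directional hit react and applies the missile damage effect from the instigator's component.
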(event `self.ReceiveBeginPlay`
  (`PrimitiveComponent.IgnoreActorWhenMoving` (`self.Sphere`) (`self.GetOwner`) true))

(event `self.Sphere.OnComponentHit`
  (params (HitComponent :type "PrimitiveComponent Object Reference") (OtherActor :type "Actor Object Reference") (OtherComp :type "PrimitiveComponent Object Reference") (NormalImpulse :type "Vector Structure") (Hit :type "HitResult Structure (by ref)"))
  (bind _returnvalue (`self.GetOwner`))
  (bind (_bblockinghit _binitialoverlap _time _distance _location _impactpoint _normal _impactnormal _physmat _hitactor) (`GameplayStatics.BreakHitResult` Hit))
  (bind _asbp_mecha_character (cast `/Game/Main/Character/BP_MechaCharacter` OtherActor)
    (:`then`
      (set `self.PlayerRef` _asbp_mecha_character)
      (`PrimitiveComponent.IgnoreActorWhenMoving` (`self.Sphere`) _returnvalue true)
      (if (== _returnvalue _hitactor)
        (`self.K2_DestroyActor`)
        (else
          (bind _output_get (set `self.TargetASC` (`AbilitySystemBlueprintLibrary.GetAbilitySystemComponent` _hitactor)))
          (`/Engine/EditorBlueprintResources/StandardMacros.IsValid` _output_get
            (:`Is Valid`
              (`MechaCharacterBase.PlayHitReactFromDirection` (`self.PlayerRef`) _impactpoint)
              (`AbilitySystemComponent.BP_ApplyGameplayEffectToTarget` :`self` (`AbilitySystemBlueprintLibrary.GetAbilitySystemComponent` (`self.GetInstigator`)) :`GameplayEffectClass` "/Game/Main/GE/Damage/Player/GE_MissleDamage.GE_MissleDamage_C" :`Target` (`self.TargetASC`) :`Level` 1.0)
              (`|SpawnActorFromClass` "/Game/Main/FX/Hit_Particle.Hit_Particle_C" (`KismetMathLibrary.MakeTransform` _impactpoint (struct) (0.6 0.6 0.6)) "Undefined" "MultiplyWithRoot" null null)
              (`self.K2_DestroyActor`))
            (:`Is Not Valid`
              (`|SpawnActorFromClass` "/Game/Main/FX/Hit_Particle.Hit_Particle_C" (`KismetMathLibrary.MakeTransform` _impactpoint (struct) (0.6 0.6 0.6)) "Undefined" "MultiplyWithRoot" null null)
              (`self.K2_DestroyActor`))))))
    (:`CastFailed`
      (`self.K2_DestroyActor`))))

(fn `UserConstructionScript`)