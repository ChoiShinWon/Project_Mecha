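; BP_MissileProjectile is a missile that flies along its local forward axis, deals damage through GAS and explodes on impact.
; On BeginPlay, ProjectileMovement drives the collision Sphere at its initial speed.
; Sphere hits ignore the owner; targets with an Ability System Component receive GE_MissleDamage from the instigator's component.
; Any other hit, with or without damage, spawns NA_Explosion2 at the impact point and destroys the missile.
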(event `self.ReceiveBeginPlay`
  (bind _projectilemovement (`self.ProjectileMovement`))
  (`MovementComponent.SetUpdatedComponent` (`self.ProjectileMovement`) (`self.Sphere`))
  (`ProjectileMovementComponent.SetVelocityInLocalSpace` _projectilemovement (`KismetMathLibrary.MakeVector` (`ProjectileMovementComponent.InitialSpeed` _projectilemovement))))

(event `self.Sphere.OnComponentHit`
  (params (HitComponent :type "PrimitiveComponent Object Reference") (OtherActor :type "Actor Object Reference") (OtherComp :type "PrimitiveComponent Object Reference") (NormalImpulse :type "Vector Structure") (Hit :type "HitResult Structure (by ref)"))
  (bind (_bblockinghit _binitialoverlap _time _distance _location _impactpoint _normal _impactnormal _physmat _hitactor) (`GameplayStatics.BreakHitResult` Hit))
  (if (not (== (`self.GetOwner`) _hitactor))
    (bind _output_get (set `self.TargetASC` (`AbilitySystemBlueprintLibrary.GetAbilitySystemComponent` _hitactor)))
    (`/Engine/EditorBlueprintResources/StandardMacros.IsValid` _output_get
      (:`Is Valid`
        (`AbilitySystemComponent.BP_ApplyGameplayEffectToTarget` :`self` (`AbilitySystemBlueprintLibrary.GetAbilitySystemComponent` (`self.GetInstigator`)) :`GameplayEffectClass` "/Game/Main/GE/Damage/GE_MissleDamage.GE_MissleDamage_C" :`Target` (`self.TargetASC`) :`Level` 1.0)
        (`|SpawnActorFromClass` "/Game/Main/Niagara/NA_Explosion2.NA_Explosion2_C" (`KismetMathLibrary.MakeTransform` _impactpoint) "Undefined" "MultiplyWithRoot" null null)
        (`self.K2_DestroyActor`))
      (:`Is Not Valid`
        (`|SpawnActorFromClass` "/Game/Main/Niagara/NA_Explosion2.NA_Explosion2_C" (`KismetMathLibrary.MakeTransform` _impactpoint) "Undefined" "MultiplyWithRoot" null null)
        (`self.K2_DestroyActor`)))))

(fn `UserConstructionScript`)