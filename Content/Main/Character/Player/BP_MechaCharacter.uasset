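; Player mecha character that fires guns and boosts through GAS ability tags and drives the mecha HUD and crosshair.
; BeginPlay creates the crosshair and starts the mission after a short delay, while Tick polls missile-cooldown and overheat tags to update the HUD.
; UI events relay mission progress and hide the HUD during cutscenes; G toggles the guide box.
; Q launches a timed zero-gravity hover with a montage, and GetBoostDirection classifies movement input using dot products.
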(event `self.ReceiveTick`
  (params (DeltaSeconds :type "Float (single-precision)"))
  (`|ExecutionSequence`
    (:`then_0`
      ;[0 0 0] 미사일 쿨타임시 글자 변경
      (if (`GameplayTagAssetInterface.HasMatchingGameplayTag` (`self.ASC`) (struct :`TagName` "Cooldown.MissileFire"))
        (`self.UpdateMissileUI` true)
        (else
          (`self.UpdateMissileUI` false))))
    (:`then_1`
      ;[0 0 0] Overheat시 글자 변경
      (if (`GameplayTagAssetInterface.HasMatchingGameplayTag` (`self.ASC`) (struct :`TagName` "State.Overheated"))
        (`self.UpdateOverHeatUI` true)
        (else
          (`self.UpdateOverHeatUI` false))))))

(event `self.ReceiveBeginPlay`
  (`parent.ReceiveBeginPlay`)
  ;[0 0 0] 크로스헤어 위젯 생성
  (bind _returnvalue (`|CreateWidget` "/Game/Main/Widget/WBP_Crosshair.WBP_Crosshair_C"))
  (bind _output_get (set `self.CrossHair` _returnvalue))
  (`UserWidget.AddToViewport` _output_get 0)
  (`KismetSystemLibrary.Delay` 0.2)
  ;[0 0 0] 미션 시작
  (bind _returnvalue_2 (`GameplayStatics.GetActorOfClass` "/Game/Main/Common/BP_MissionManager.BP_MissionManager_C"))
  (`MissionManager.StartMission` _returnvalue_2))

(event `Key|G`
  (params (Key :type "Key Structure"))
  ;[1 1 1] 가이드 창 숨기고 키기
  (:`Pressed`
    (if (`self.IsGuideBoxShow`)
      (bind _aswbp_mecha_hud2 (cast `/Game/Main/Widget/WBP_MechaHUD2` (`self.MechaHUDWidget`)))
      (`/Game/Main/Widget/WBP_MechaHUD2.HideGuideBox` _aswbp_mecha_hud2)
      (set `self.IsGuideBoxShow` false)
      (else
        (bind _aswbp_mecha_hud2_2 (cast `/Game/Main/Widget/WBP_MechaHUD2` (`self.MechaHUDWidget`)))
        (`/Game/Main/Widget/WBP_MechaHUD2.ShowGuideBox` _aswbp_mecha_hud2_2)
        (set `self.IsGuideBoxShow` true)))))

(event `EnhancedInput|/Game/Main/IA/IA_GunFire`
  (params (ActionValue :type Boolean) (ElapsedSeconds :type "Float (double-precision)") (TriggeredSeconds :type "Float (double-precision)") (InputAction :type "InputAction Object Reference" :default "/Game/Main/IA/IA_GunFire.IA_GunFire"))
  ;[0 0 0] 총 발사 (RMB)
  (:`Ongoing`
    (`AbilitySystemComponent.TryActivateAbilitiesByTag` (`self.AbilitySystem`) (`BlueprintGameplayTagLibrary.MakeGameplayTagContainerFromTag` (struct :`TagName` "Ability.GunFire")) true)))

(event `EnhancedInput|/Game/Main/IA/IA_BoostMode`
  (params (ActionValue :type Boolean) (ElapsedSeconds :type "Float (double-precision)") (TriggeredSeconds :type "Float (double-precision)") (InputAction :type "InputAction Object Reference" :default "/Game/Main/IA/IA_BoostMode.IA_BoostMode"))
  (:`Started`
    (`AbilitySystemComponent.TryActivateAbilitiesByTag` (`self.AbilitySystem`) (`BlueprintGameplayTagLibrary.MakeGameplayTagContainerFromTag` (struct :`TagName` "Ability.Boost")) true)
    ;[0 0 0] UI에 부스트 글자 출력
    (bind _aswbp_mecha_hud2 (cast `/Game/Main/Widget/WBP_MechaHUD2` (`self.MechaHUDWidget`)))
    (`/Game/Main/Widget/WBP_MechaHUD2.Boost Set` _aswbp_mecha_hud2 (`self.IsBoost`))))

(event `MissionStartedUI`
  (params (RequiredKillCount :type Integer))
  (bind _mechahudwidget (`self.MechaHUDWidget`))
  ;[0 0 0] UI연동
  (`/Engine/EditorBlueprintResources/StandardMacros.IsValid` _mechahudwidget
    (:`Is Valid`
      (bind _aswbp_mecha_hud2 (cast `/Game/Main/Widget/WBP_MechaHUD2` _mechahudwidget))
      (`/Game/Main/Widget/WBP_MechaHUD2.MissionStarted` _aswbp_mecha_hud2 RequiredKillCount))))

(event `MissionProgress_UI`
  (params (CurrentKillCount :type Integer) (RequiredKillCount :type Integer))
  (bind _mechahudwidget (`self.MechaHUDWidget`))
  ;[0 0 0] UI연동
  (`/Engine/EditorBlueprintResources/StandardMacros.IsValid` _mechahudwidget
    (:`Is Valid`
      (bind _aswbp_mecha_hud2 (cast `/Game/Main/Widget/WBP_MechaHUD2` _mechahudwidget))
      (`/Game/Main/Widget/WBP_MechaHUD2.MissionProgress` _aswbp_mecha_hud2 CurrentKillCount RequiredKillCount))))

(event `Key|Q`
  (params (Key :type "Key Structure"))
  (:`Pressed`
    (set `CharacterMovementComponent.GravityScale` 0.0 (`self.CharacterMovement`))
    (`self.Jump`)
    (`self.LaunchCharacter` (0.0 0.0 700.0))
    (`self.StopJumping`)
    (`self.PlayAnimMontage` "/Game/Main/Anim/Boss/AM_Boss_MissileRain.AM_Boss_MissileRain")
    (`KismetSystemLibrary.Delay` 5.0)
    (set `CharacterMovementComponent.GravityScale` 3.0 (`self.CharacterMovement`))))

(event `CutsceneStart`
  (bind _mechahudwidget (`self.MechaHUDWidget`))
  (`/Engine/EditorBlueprintResources/StandardMacros.IsValid` _mechahudwidget
    (:`Is Valid`
      (bind _aswbp_mecha_hud2 (cast `/Game/Main/Widget/WBP_MechaHUD2` _mechahudwidget))
      ;[0 0 0] 컷신 시작시 UI 숨김
      (`/Game/Main/Widget/WBP_MechaHUD2.SetHUDVisible` _aswbp_mecha_hud2 false)
      (`/Game/Main/Widget/WBP_MechaHUD2.HideMission` _aswbp_mecha_hud2)
      (`/Game/Main/Widget/WBP_Crosshair.SetCrosshairVisible` (`self.CrossHair`) false))))

(event `CutsceneEnd`
  (bind _mechahudwidget (`self.MechaHUDWidget`))
  (`/Engine/EditorBlueprintResources/StandardMacros.IsValid` _mechahudwidget
    (:`Is Valid`
      (bind _aswbp_mecha_hud2 (cast `/Game/Main/Widget/WBP_MechaHUD2` _mechahudwidget))
      ;[0 0 0] 컷신 종료후  UI 다시 표시
      (`/Game/Main/Widget/WBP_MechaHUD2.SetHUDVisible` _aswbp_mecha_hud2 true)
      (`/Game/Main/Widget/WBP_Crosshair.SetCrosshairVisible` (`self.CrossHair`) true))))

(event `UpdateOverHeatUI`
  (params (IsOverHeat :type Boolean))
  (bind _mechahudwidget (`self.MechaHUDWidget`))
  (`/Engine/EditorBlueprintResources/StandardMacros.IsValid` _mechahudwidget
    (:`Is Valid`
      (bind _aswbp_mecha_hud2 (cast `/Game/Main/Widget/WBP_MechaHUD2` _mechahudwidget))
      (if IsOverHeat
        (`/Game/Main/Widget/WBP_MechaHUD2.ShowOverHeat` _aswbp_mecha_hud2)
        (else
          (`/Game/Main/Widget/WBP_MechaHUD2.HideOverHeat` _aswbp_mecha_hud2))))))

(event `UpdateMissileUI`
  (params (IsReloading :type Boolean))
  (bind _mechahudwidget (`self.MechaHUDWidget`))
  (`/Engine/EditorBlueprintResources/StandardMacros.IsValid` _mechahudwidget
    (:`Is Valid`
      (bind _aswbp_mecha_hud2 (cast `/Game/Main/Widget/WBP_MechaHUD2` _mechahudwidget))
      (if IsReloading
        (`/Game/Main/Widget/WBP_MechaHUD2.ShowMissile` _aswbp_mecha_hud2)
        (else
          (`/Game/Main/Widget/WBP_MechaHUD2.HideMissile` _aswbp_mecha_hud2))))))

(fn `Get Boost Direction`
  (returns (Direction :type Name))
  (bind _returnvalue (`GameplayStatics.GetPlayerPawn` 0))
  (bind _returnvalue_2 (`self.GetLastMovementInputVector` _returnvalue))
  (bind _returnvalue_3 (`KismetMathLibrary.Dot_VectorVector` (`self.GetActorRightVector` _returnvalue) _returnvalue_2))
  (bind _returnvalue_4 (`KismetMathLibrary.Dot_VectorVector` (`self.GetActorForwardVector` _returnvalue) _returnvalue_2))
  (bind _asbp_mecha_character (cast `/Game/Main/Character/Player/BP_MechaCharacter` _returnvalue))
  (set `self.Char` _asbp_mecha_character)
  (if (> _returnvalue_4 0.7)
    ;[0 0 0] 전방 방향 설정
    (bind _output_get (set `/Game/Main/Character/Player/BP_MechaCharacter.CurrentBoostDirection` "Forward" (`self.Char`)))
    (return _output_get)
    (elif (< _returnvalue_4 -0.7)
      ;[0 0 0] 후방
      (bind _output_get_2 (set `/Game/Main/Character/Player/BP_MechaCharacter.CurrentBoostDirection` "BackWard" (`self.Char`)))
      (return _output_get_2)
      (elif (> _returnvalue_3 0.7)
        ;[0 0 0] 우측
        (bind _output_get_3 (set `/Game/Main/Character/Player/BP_MechaCharacter.CurrentBoostDirection` "Right" (`self.Char`)))
        (return _output_get_3)
        (elif (< _returnvalue_3 -0.7)
          ;[0 0 0] 좌측
          (bind _output_get_4 (set `/Game/Main/Character/Player/BP_MechaCharacter.CurrentBoostDirection` "Left" (`self.Char`)))
          (return _output_get_4))))))

(fn `UserConstructionScript`)