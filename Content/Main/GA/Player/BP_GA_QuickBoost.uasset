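; Quick boost gameplay ability that launches the player mecha in its movement input direction.
; It stores the boost direction, zeroes gravity and sets Flying before committing, then projects last input onto control-yaw axes for the launch.
; After a brief delay it applies the energy-drain effect, restores gravity and ends.
; Flying is never reset here; failed commit leaves gravity at zero, and missing input also leaves the ability active.
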(event `self.K2_ActivateAbility`
  (bind _asbp_mecha_character (cast `/Game/Main/Character/Player/BP_MechaCharacter` (`GameplayStatics.GetPlayerPawn` 0))
    (:`then`
      ;[1 1 1] 캐릭터 BP에 있는 함수
      (bind _direction (`/Game/Main/Character/Player/BP_MechaCharacter.Get Boost Direction` _asbp_mecha_character))
      (set `/Game/Main/Character/Player/BP_MechaCharacter.CurrentBoostDirection` _direction _asbp_mecha_character)
      (set `self.Char` _asbp_mecha_character)
      (bind _charactermovement (`Character.CharacterMovement` _asbp_mecha_character))
      ;[1 1 1] 퀵부스트시 중력 0
      (set `CharacterMovementComponent.GravityScale` 0.0 _charactermovement)
      (`CharacterMovementComponent.SetMovementMode` _charactermovement "MOVE_Flying" 0)
      (bind _returnvalue (`self.K2_CommitAbility`))
      (if _returnvalue
        (bind _asbp_mecha_character_2 (cast `/Game/Main/Character/Player/BP_MechaCharacter` (`self.GetAvatarActorFromActorInfo`)))
        (bind _output_get (set `self.Char` _asbp_mecha_character_2))
        (bind _returnvalue_2 (`PawnMovementComponent.GetLastInputVector` (`Character.CharacterMovement` _asbp_mecha_character_2)))
        (if (> (`KismetMathLibrary.VSize` _returnvalue_2) 0.1)
          (bind _returnvalue_3 (`KismetMathLibrary.MakeRotator` 0.0 0.0 (.yaw (`Controller.GetControlRotation` (`Pawn.GetController` _output_get)))))
          (bind _returnvalue_4 (`KismetMathLibrary.GetForwardVector` _returnvalue_3))
          (bind _returnvalue_5 (`KismetMathLibrary.Vector_Normal2D` _returnvalue_2))
          (bind _returnvalue_6 (`KismetMathLibrary.GetRightVector` _returnvalue_3))
          (`Character.LaunchCharacter` (`self.Char`) (+ (* (`KismetMathLibrary.Normal` (+ (* _returnvalue_4 (`KismetMathLibrary.Dot_VectorVector` _returnvalue_4 _returnvalue_5)) (* _returnvalue_6 (`KismetMathLibrary.Dot_VectorVector` _returnvalue_6 _returnvalue_5)))) (`self.LaunchXY`)) (`KismetMathLibrary.MakeVector` 0.0 0.0 (`self.LaunchZ`))) true false)
          (`KismetSystemLibrary.Delay` 0.05)
          ;[1 1 1] 순간 스피드를 올리고 에너지 소모
          (`self.BP_ApplyGameplayEffectToOwner` "/Game/Main/GE/Player/GE_QuickBoostDrain.GE_QuickBoostDrain_C")
          ;[1 1 1] 중력 다시 복구
          (set `CharacterMovementComponent.GravityScale` 1.0 (`Character.CharacterMovement` (`self.Char`)))
          (`self.K2_EndAbility`))
        (else
          (`self.K2_EndAbility`))))
    (:`CastFailed`
      (`self.K2_EndAbility`))))

(event `self.K2_OnEndAbility`
  (params (bWasCancelled :type Boolean)))