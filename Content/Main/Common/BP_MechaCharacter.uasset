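; Player mecha character that turns Enhanced Input actions into movement and combat abilities and adds a crosshair widget on BeginPlay.
; Boost, dash, melee, missile, gun and reload inputs activate Gameplay Abilities by tag, while holding jump sets an airborne flag.
; OnBoostChanged stores the boost state, which the boost toggle passes to the mecha HUD.
; GetBoostDirection compares player 0's last movement input with its facing using dot products to pick one of four directions.
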(event `EnhancedInput|/Game/Main/Input_Action/IA_Jump_Mecha`
  (params (ActionValue :type Boolean) (ElapsedSeconds :type "Float (double-precision)") (TriggeredSeconds :type "Float (double-precision)") (InputAction :type "InputAction Object Reference" :default "/Game/Main/Input_Action/IA_Jump_Mecha.IA_Jump_Mecha"))
  (:`Ongoing`
    (set `self.IsOnAir` true))
  (:`Canceled`
    (set `self.IsOnAir` false)))

(event `self.ReceiveBeginPlay`
  ;[1 1 1] 크로스헤어 위젯 생성
  (bind _returnvalue (`|CreateWidget` "/Game/Main/Widget/WBP_Crosshair.WBP_Crosshair_C"))
  (`UserWidget.AddToViewport` _returnvalue 0))

(event `EnhancedInput|/Game/Main/Input_Action/IA_Sprint_Mecha`
  (params (ActionValue :type Boolean) (ElapsedSeconds :type "Float (double-precision)") (TriggeredSeconds :type "Float (double-precision)") (InputAction :type "InputAction Object Reference" :default "/Game/Main/Input_Action/IA_Sprint_Mecha.IA_Sprint_Mecha"))
  ;[1 1 1] 퀵부스트 (Left Shift
  (:`Started`
    (`AbilitySystemComponent.TryActivateAbilitiesByTag` (`self.AbilitySystem`) (`BlueprintGameplayTagLibrary.MakeGameplayTagContainerFromTag` (struct :`TagName` "Ability.QuickBoost")) true)))

(event `EnhancedInput|/Game/Main/Input_Action/IA_BoostMode`
  (params (ActionValue :type Boolean) (ElapsedSeconds :type "Float (double-precision)") (TriggeredSeconds :type "Float (double-precision)") (InputAction :type "InputAction Object Reference" :default "/Game/Main/Input_Action/IA_BoostMode.IA_BoostMode"))
  ;[1 1 1] 부스트모드  On/Off (B)
  (:`Started`
    (`AbilitySystemComponent.TryActivateAbilitiesByTag` (`self.AbilitySystem`) (`BlueprintGameplayTagLibrary.MakeGameplayTagContainerFromTag` (struct :`TagName` "Ability.Boost")) true)
    (bind _aswbp_mecha_hud2 (cast `/Game/Main/Widget/WBP_MechaHUD2` (`self.MechaHUDWidget`)))
    (`/Game/Main/Widget/WBP_MechaHUD2.Boost Set` _aswbp_mecha_hud2 (`self.IsBoost`))))

(event `OnBoostChanged`
  (params (BoostActive :type Boolean))
  (set `self.IsBoost` BoostActive))

(event `EnhancedInput|/Game/Main/Input_Action/IA_Attack`
  (params (ActionValue :type Boolean) (ElapsedSeconds :type "Float (double-precision)") (TriggeredSeconds :type "Float (double-precision)") (InputAction :type "InputAction Object Reference" :default "/Game/Main/Input_Action/IA_Attack.IA_Attack"))
  ;[1 1 1] 근접 공격 (LMB)
  (:`Started`
    (`AbilitySystemComponent.TryActivateAbilitiesByTag` (`self.AbilitySystem`) (`BlueprintGameplayTagLibrary.MakeGameplayTagContainerFromTag` (struct :`TagName` "Ability.Attack")) true)))

(event `EnhancedInput|/Game/Main/Input_Action/IA_AssaultBoost`
  (params (ActionValue :type Boolean) (ElapsedSeconds :type "Float (double-precision)") (TriggeredSeconds :type "Float (double-precision)") (InputAction :type "InputAction Object Reference" :default "/Game/Main/Input_Action/IA_AssaultBoost.IA_AssaultBoost"))
  ;[1 1 1] 어썰트부스트 (Ctrl)
  (:`Started`
    (`AbilitySystemComponent.TryActivateAbilitiesByTag` (`self.AbilitySystem`) (`BlueprintGameplayTagLibrary.MakeGameplayTagContainerFromTag` (struct :`TagName` "Ability.AssaultBoost")) true)))

(event `EnhancedInput|/Game/Main/Input_Action/IA_MissileFire`
  (params (ActionValue :type Boolean) (ElapsedSeconds :type "Float (double-precision)") (TriggeredSeconds :type "Float (double-precision)") (InputAction :type "InputAction Object Reference" :default "/Game/Main/Input_Action/IA_MissileFire.IA_MissileFire"))
  ;[1 1 1] 미사일 발사 (E)
  (:`Started`
    (`AbilitySystemComponent.TryActivateAbilitiesByTag` (`self.AbilitySystem`) (`BlueprintGameplayTagLibrary.MakeGameplayTagContainerFromTag` (struct :`TagName` "Ability.MissileFire")) true)))

(event `EnhancedInput|/Game/Main/Input_Action/IA_GunFire`
  (params (ActionValue :type Boolean) (ElapsedSeconds :type "Float (double-precision)") (TriggeredSeconds :type "Float (double-precision)") (InputAction :type "InputAction Object Reference" :default "/Game/Main/Input_Action/IA_GunFire.IA_GunFire"))
  ;[1 1 1] 총 발사 (RMB)
  (:`Ongoing`
    (`AbilitySystemComponent.TryActivateAbilitiesByTag` (`self.AbilitySystem`) (`BlueprintGameplayTagLibrary.MakeGameplayTagContainerFromTag` (struct :`TagName` "Ability.GunFire")) true)))

(event `EnhancedInput|/Game/Main/Input_Action/IA_Reload`
  (params (ActionValue :type Boolean) (ElapsedSeconds :type "Float (double-precision)") (TriggeredSeconds :type "Float (double-precision)") (InputAction :type "InputAction Object Reference" :default "/Game/Main/Input_Action/IA_Reload.IA_Reload"))
  ;[1 1 1] 장전
  (:`Started`
    (`AbilitySystemComponent.TryActivateAbilitiesByTag` (`self.AbilitySystem`) (`BlueprintGameplayTagLibrary.MakeGameplayTagContainerFromTag` (struct :`TagName` "Ability.Reload")) true)))

(fn `Get Boost Direction`
  (returns (Direction :type Name))
  (bind _returnvalue (`GameplayStatics.GetPlayerPawn` 0))
  (bind _returnvalue_2 (`self.GetLastMovementInputVector` _returnvalue))
  (bind _returnvalue_3 (`KismetMathLibrary.Dot_VectorVector` (`self.GetActorRightVector` _returnvalue) _returnvalue_2))
  (bind _returnvalue_4 (`KismetMathLibrary.Dot_VectorVector` (`self.GetActorForwardVector` _returnvalue) _returnvalue_2))
  (bind _asbp_mecha_character (cast `/Game/Main/Common/BP_MechaCharacter` _returnvalue))
  (set `self.Char` _asbp_mecha_character)
  (if (> _returnvalue_4 0.7)
    ;[1 1 1] 전방 방향 설정
    (bind _output_get (set `/Game/Main/Common/BP_MechaCharacter.CurrentBoostDirection` "Forward" (`self.Char`)))
    (return _output_get)
    (elif (< _returnvalue_4 -0.7)
      ;[1 1 1] 후방
      (bind _output_get_2 (set `/Game/Main/Common/BP_MechaCharacter.CurrentBoostDirection` "BackWard" (`self.Char`)))
      (return _output_get_2)
      (elif (> _returnvalue_3 0.7)
        ;[1 1 1] 우측
        (bind _output_get_3 (set `/Game/Main/Common/BP_MechaCharacter.CurrentBoostDirection` "Right" (`self.Char`)))
        (return _output_get_3)
        (else
          ;[1 1 1] 좌측
          (if (< _returnvalue_3 -0.7)
            (bind _output_get_4 (set `/Game/Main/Common/BP_MechaCharacter.CurrentBoostDirection` "Left" (`self.Char`)))
            (return _output_get_4)))))))

(fn `UserConstructionScript`)