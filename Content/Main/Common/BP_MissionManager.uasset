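; Mission manager actor that relays mission state to the player's BP_MechaCharacter and stages the boss introduction.
; Mission start and progress events forward kill counts to the character's UI functions.
; The boss phase disables pawn input and plays the intro sequence between cutscene start and end calls.
; A fixed delay, rather than a sequence-finished callback, restores input and spawns BP_BossCrunch at the manager's transform, storing its reference.
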(event `self.OnMissionStartedBP`
  (params (InRequiredKillCount :type Integer))
  (bind _asbp_mecha_character (cast `/Game/Main/Character/Player/BP_MechaCharacter` (`GameplayStatics.GetPlayerCharacter` 0)))
  (`/Game/Main/Character/Player/BP_MechaCharacter.MissionStartedUI` _asbp_mecha_character InRequiredKillCount))

(event `self.OnMissionProgressBP`
  (params (InCurrentKillCount :type Integer) (InRequiredKillCount :type Integer))
  (bind _asbp_mecha_character (cast `/Game/Main/Character/Player/BP_MechaCharacter` (`GameplayStatics.GetPlayerCharacter` 0)))
  (`/Game/Main/Character/Player/BP_MechaCharacter.MissionProgress_UI` _asbp_mecha_character InCurrentKillCount InRequiredKillCount))

(event `self.OnBossPhaseStartedBP`
  (bind _returnvalue (`GameplayStatics.GetPlayerController` 0))
  (bind _returnvalue_2 (`Controller.K2_GetPawn` _returnvalue))
  (bind _asbp_mecha_character (cast `/Game/Main/Character/Player/BP_MechaCharacter` _returnvalue_2))
  (bind _output_get (set `self.PlayerPawn` _returnvalue_2))
  (`self.DisableInput` _output_get _returnvalue)
  (`/Game/Main/Character/Player/BP_MechaCharacter.CutsceneStart` _asbp_mecha_character)
  (`MovieSceneSequencePlayer.Play` (`LevelSequenceActor.SequencePlayer` (`self.BossIntroSequenceActor`)))
  (`KismetSystemLibrary.Delay` 7.0)
  (`/Game/Main/Character/Player/BP_MechaCharacter.CutsceneEnd` _asbp_mecha_character)
  (`self.EnableInput` (`self.PlayerPawn`) (`GameplayStatics.GetPlayerController` 0))
  (bind _returnvalue_3 (`|SpawnActorFromClass` :`Class` "/Game/Main/Character/Enemy/BP_BossCrunch.BP_BossCrunch_C" :`SpawnTransform` (`self.GetTransform`) :`CollisionHandlingOverride` "Undefined" :`TransformScaleMethod` "MultiplyWithRoot" :`PlayerRef` null :`Instigator` null))
  (bind _output_get_2 (set `self.BossRef` _returnvalue_3))
  (set `self.BossInstance` _output_get_2))

(fn `UserConstructionScript`)